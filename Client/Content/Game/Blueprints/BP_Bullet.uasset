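; Bullet projectile actor that flies visually from its spawn point to a given end location.
; StartMoving plays a timeline at the passed Speed as play rate, lerping the actor's position without sweeping, or destroys it if SpawnBullet is false.
; Each update runs a small zero-length Visibility sphere trace at the bullet mesh, destroying the actor on a hit or when the timeline finishes.
; BeginPlay adds a one-second lifetime fallback.
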(event Custom|Start%20Moving
  (params (Spawn%20Bullet :type Boolean) (End%20Location :type Vector) (Speed :type Float%20%28single-precision%29) (Attach%20Component :type Scene%20Component%20Object%20Reference) (Attach%20Socket%20Name :type Name))
  (bind _bulletm4a1 (Variables|Default|GetBulletM4A1))
  (bind _returnvalue (Transformation|GetWorldLocation _bulletm4a1))
  (if Spawn%20Bullet
    (Components|Timeline|SetPlayRate (Variables|Default|GetTL) Speed)
    (Variables|Default|SetEnd%20Location End%20Location)
    (Variables|Default|SetStart%20Location (Transformation|GetActorLocation))
    (bind _alpha (Timeline|TL PlayFromStart)
      (:Update
        (Transformation|SetActorLocation (Math|Vector|Lerp(Vector) (Variables|Default|GetStart%20Location) (Variables|Default|GetEnd%20Location) _alpha) false false)
        (bind _returnvalue_2 (Collision|SphereTraceByChannel _returnvalue _returnvalue 1e+01 "TraceTypeQuery1" false 0 "None"))
        (if _returnvalue_2
          (CallFunction|Stop)
          (Actor|DestroyActor)))
      (:Finished
        (CallFunction|Stop)
        (Actor|DestroyActor)))
    (else
      (Actor|DestroyActor))))

(event Custom|Stop
  (bind _bulletm4a1 (Variables|Default|GetBulletM4A1))
  (bind _returnvalue (Transformation|GetWorldLocation _bulletm4a1))
  (bind _alpha (Timeline|TL Stop)
    (:Update
      (Transformation|SetActorLocation (Math|Vector|Lerp(Vector) (Variables|Default|GetStart%20Location) (Variables|Default|GetEnd%20Location) _alpha) false false)
      (bind _returnvalue_2 (Collision|SphereTraceByChannel _returnvalue _returnvalue 1e+01 "TraceTypeQuery1" false 0 "None"))
      (if _returnvalue_2
        (CallFunction|Stop)
        (Actor|DestroyActor)))
    (:Finished
      (CallFunction|Stop)
      (Actor|DestroyActor))))

(event EventBeginPlay
  (Utilities|FlowControl|Delay 1.0)
  (Utilities|IsValid self
    (:Is%20Valid
      (Actor|DestroyActor))))

(fn ConstructionScript)