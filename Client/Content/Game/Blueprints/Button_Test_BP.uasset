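; Test actor that shows a point light while a referenced button actor is pressed and hides it otherwise.
; Tick polls the button's IsPressed state through a DoOnceBranch, which sets the light's visibility on each branch.
; BeginPlay disables ticking when no valid button actor is assigned.
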(event EventBeginPlay
  (Utilities|IsValid (Variables|Default|GetButton%20Actor)
    (:Is%20Not%20Valid
      (Actor|Tick|SetActorTickEnabled false))))

(event EventTick
  (params (DeltaSeconds :type Float%20%28single-precision%29))
  (Utilities|DoOnceBranch (Variables|/Game/Game/Blueprints/BP_I_Button.BP_I_Button_C|GetIs%20Pressed (Variables|Default|GetButton%20Actor))
    (:True
      (Rendering|SetVisibility (Variables|Default|GetPointLight) true false))
    (:False
      (Rendering|SetVisibility (Variables|Default|GetPointLight) false false))))

(fn ConstructionScript)