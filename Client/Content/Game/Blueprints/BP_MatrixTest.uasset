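; Test actor that checks world-to-local and local-to-world matrix transform conversion on a Cube component.
; On BeginPlay it traces toward the cube's center, builds a transform from the hit point and normal, and stores it in cube-local space.
; Tick converts it back to world space and draws a debug arrow, so the point follows the cube.
; A timeline to animate the cube's transform exists but never runs.
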(event EventBeginPlay
  (bind _cube (Variables|Default|GetCube))
  (bind _returnvalue (Transformation|GetWorldLocation _cube))
  (bind (_outhit _returnvalue_2) (Collision|LineTraceByChannel (+ _returnvalue (* (Math|Vector|GetForwardVector _cube) (* (Math|Vector|VectorLength (Transformation|GetActorScale3D)) 5e+01))) _returnvalue "TraceTypeQuery1" false 0 "ForDuration" false "(R=1.000000,G=0.000000,B=0.000000,A=1.000000)" "(R=0.000000,G=1.000000,B=0.000000,A=1.000000)" 2.0))
  (if _returnvalue_2
    (Variables|Default|SetPointWS (Math|Transform|MakeTransform (.ImpactPoint (Collision|BreakHitResult _outhit)) (Math|Rotator|MakeRotfromX (* (.Normal (Collision|BreakHitResult _outhit)) -1.0))))
    (Variables|Default|SetPointLS (* (Math|Transform|ToMatrix(Transform) (Variables|Default|GetPointWS)) (Class|KismetMathLibrary|MatrixGetInverse (Math|Transform|ToMatrix(Transform) (Transformation|GetWorldTransform (Variables|Default|GetCube))))))
    (Variables|Default|SetTPointLS (Math|Conversions|ToTransform(Vector) (* (Math|Transform|ToMatrix(Transform) (Variables|Default|GetPointWS)) (Class|KismetMathLibrary|MatrixGetInverse (Math|Transform|ToMatrix(Transform) (Transformation|GetWorldTransform (Variables|Default|GetCube)))))))
    (Variables|Default|SetLocal%20Space%20Component (Utilities|Struct|MakeALS_ComponentAndTransform (.transform (CallFunction|FLWorldtoLocal(Matrix) (Utilities|Struct|MakeALS_ComponentAndTransform (Variables|Default|GetPointWS) (Variables|Default|GetCube)))) (.component (CallFunction|FLWorldtoLocal(Matrix) (Utilities|Struct|MakeALS_ComponentAndTransform (Variables|Default|GetPointWS) (Variables|Default|GetCube))))))))

(event EventTick
  (params (DeltaSeconds :type Float%20%28single-precision%29))
  (bind _local_space_component (Variables|Default|GetLocal%20Space%20Component))
  (bind _world (CallFunction|FLLocaltoWorld(Matrix) _local_space_component))
  (Rendering|Debug|DrawDebugArrow (.location (.transform _world)) (+ (.location (.transform _world)) (* (Math|Vector|GetForwardVector (.rotation (.transform _world))) -3e+01)) 15.0 "(R=1.000000,G=0.091393,B=0.000000,A=1.000000)" 0.0 2.0))

(fn ConstructionScript)