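; Lobby player controller that switches input mode and mouse cursor visibility for the main menu.
; UpdateInputMode acts only when given a valid widget, setting cursor visibility and choosing Game and UI focused on that widget, or Game Only with the mouse moved to the origin.
; A local OnceBranch macro pairs two cross-resetting DoOnce nodes, intended to avoid reapplying an unchanged mode.
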(event Custom|UpdateInputMode
  (params (ShowMouseCursor :type Boolean) (InWidgetToFocus :type Widget%20Object%20Reference))
  (bind _self self)
  ;[0 0 0] Update Input Mode
  (if (Utilities|IsValid InWidgetToFocus)
    (bind _output_get (Variables|Default|SetbShowMouseCursor ShowMouseCursor))
    (Utilities|OnceBranch _output_get
      (:True
        (Input|SetInputModeGameandUI _self InWidgetToFocus "DoNotLock" true))
      (:False
        (Input|SetInputModeGameOnly _self)
        (Class|PlayerController|SetMouseLocation)))))

(fn ConstructionScript)