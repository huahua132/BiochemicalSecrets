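; Team PVP game mode that assigns joining players to Blue or Red and spawns their characters at team spawn points.
; On join, it sorts PlayerStarts by tag into team arrays and sets the player's number from the PlayerArray size.
; It puts the player on the smaller team in GS_Game, ties going to Blue, and stores the side in PS_Game.
; SpawnCharacterAndControl then uses a random start from that team.
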(event Custom|SpawnCharacter
  (params (PlayerController :type Player%20Controller%20Object%20Reference))
  (bind _buleteam (Variables|Default|GetBuleTeam))
  (bind _redteam (Variables|Default|GetRedTeam))
  ;[1 1 1] 创建默认玩家
  (bind _asps_game (Utilities|Casting|CastToPS_Game (Variables|/Script/Engine.Controller|GetPlayerState PlayerController))
    (:then
      (if (Variables|/Game/Blueprints/PS_Game.PS_Game_C|GetIsBlue? _asps_game)
        (CallFunction|SpawnCharacterandControl PlayerController (Transformation|GetActorTransform (Utilities|Array|Get(acopy) _buleteam (Math|Random|RandomInteger (Utilities|Array|Length _buleteam)))))
        (else
          (CallFunction|SpawnCharacterandControl PlayerController (Transformation|GetActorTransform (Utilities|Array|Get(acopy) _redteam (Math|Random|RandomInteger (Utilities|Array|Length _redteam))))))))
    (:CastFailed
      (Development|PrintString "Cast To PS Game Failed!" true true "(R=1.000000,G=0.055457,B=0.000000,A=1.000000)" 6e+01))))

(event EventBeginPlay
  (|CallParentFunction) ; This node is disabled and will not be called.\nDrag off pins to build functionality.
)

(event EventTick
  (params (DeltaSeconds :type Float%20%28single-precision%29))
  (|CallParentFunction DeltaSeconds) ; This node is disabled and will not be called.\nDrag off pins to build functionality.
)

(event EventOnNewPlayerJoin
  (params (PlayerController :type Player%20Controller%20Object%20Reference) (Guid :type String) (Character :type Integer) (Name :type String) (Team :type Integer))
  (Development|PrintString "新玩家加入")
  (CallFunction|CharacterInit PlayerController)
  (CallFunction|SpawnCharacter PlayerController))

(fn ConstructionScript
  (|CallParentFunction))

(fn GetModuleName
  (return "Game/GM_PVP_Team"))

(fn CharacterInit
  (params (PlayerController :type Player%20Controller%20Object%20Reference))
  ;[1 0.581 0.2476 0.8365] 分配阵营
  (Utilities|FlowControl|Sequence
    (:then_0
      (bind _outactors (Actor|GetAllActorsOfClass "/Script/Engine.PlayerStart"))
      (for _array_element _outactors
        (if (Utilities|Name|Equal(Name) (Variables|/Script/Engine.PlayerStart|GetPlayerStartTag _array_element) "Blue")
          (Utilities|Array|AddUnique (Variables|Default|GetBuleTeam) _array_element)
          (elif (Utilities|Name|Equal(Name) (Variables|/Script/Engine.PlayerStart|GetPlayerStartTag _array_element) "Red")
            (Utilities|Array|AddUnique (Variables|Default|GetRedTeam) _array_element))))
      (bind _asps_game (Utilities|Casting|CastToPS_Game (Variables|/Script/Engine.Controller|GetPlayerState PlayerController)))
      (Variables|/Game/Blueprints/PS_Game.PS_Game_C|SetPlayerNumber _asps_game (Utilities|Array|Length (Variables|/Script/Engine.GameState|GetPlayerArray (Game|GetGameState)))))
    (:then_1
      (bind _asgs_game (Utilities|Casting|CastToGS_Game (Game|GetGameState)))
      (bind _asps_game_2 (Utilities|Casting|CastToPS_Game (Variables|/Script/Engine.Controller|GetPlayerState PlayerController)))
      (bind _output_get (Variables|/Game/Blueprints/PS_Game.PS_Game_C|SetIsBlue? _asps_game_2 (<= (Utilities|Array|Length (Variables|/Game/Blueprints/GS_Game.GS_Game_C|GetPlayerBlue _asgs_game)) (Utilities|Array|Length (Variables|/Game/Blueprints/GS_Game.GS_Game_C|GetPlayerRed _asgs_game)))))
      (if _output_get
        ;;[1 1 1] blue
        (Utilities|Array|AddUnique (Variables|/Game/Blueprints/GS_Game.GS_Game_C|GetPlayerBlue _asgs_game) PlayerController)
        (else
          ;;[1 1 1] Red
          (Utilities|Array|AddUnique (Variables|/Game/Blueprints/GS_Game.GS_Game_C|GetPlayerRed _asgs_game) PlayerController))))))