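; GM_Login is the login level's game mode, which starts the client and shows the login interface for the current platform.
; On BeginPlay it has the game instance create its tick event actor and run ClientMain, then calls ShowLoginUI.
; PC and Mobile show a cached WB_Login widget with the mouse cursor enabled.
; VR instead possesses a UI_Pawn spawned at the PlayerStart and spawns a 3D main-menu HUD actor for interaction.
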(event EventBeginPlay
  (bind _g_instance (CallFunction|GetInstance))
  ;[1 1 1] 初始化实例
  (Default|GenerateTickEventActor _g_instance)
  (Default|ClientMain _g_instance)
  (CallFunction|ShowLoginUI))

(event EventTick
  (params (DeltaSeconds :type Float%20%28single-precision%29)))

(fn ConstructionScript)

(fn ShowLoginUI
  ;[1 1 1] VR平台创建UI Pawn进行交互
  (switch Utilities|FlowControl|Switch|SwitchonPlatformGroup (Variables|/Game/Blueprints/G_Instance.G_Instance_C|GetPlatform (CallFunction|GetInstance))
    (:NewEnumerator1
      (CallFunction|CreateUI :!label _label))
    (:NewEnumerator3
      (goto _label))
    (:NewEnumerator4
      (bind _returnvalue (Actor|GetActorOfClass "/Script/Engine.PlayerStart"))
      (bind _returnvalue_2 (Game|SpawnActorfromClass "/Game/Blueprints/UI_Pawn.UI_Pawn_C" (Transformation|GetActorTransform _returnvalue) "Undefined" 0 0))
      (Pawn|Possess (Game|GetPlayerController 0) _returnvalue_2)
      (Game|SpawnActorfromClass "/Game/Lobby/Blueprints/MainMenu/BP_3D_HUD_MainMenu.BP_3D_HUD_MainMenu_C" (Math|Transform|MakeTransform "0, 0, 0") "Undefined" 0 0))))

(fn CreateUI
  (Variables|/Script/Engine.PlayerController|SetbShowMouseCursor (Game|GetPlayerController 0) true)
  (Utilities|IsValid (Variables|Default|GetWB_Login)
    (:Is%20Valid
      _)
    (:Is%20Not%20Valid
      (bind _returnvalue (UserInterface|CreateWidget "/Game/Lobby/Widgets/WB_Login.WB_Login_C"))
      (bind _output_get (Variables|Default|SetWB_Login _returnvalue))))
  (UserInterface|Viewport|AddtoViewport _output_get 0)
  (return (Variables|Default|GetWB_Login)))